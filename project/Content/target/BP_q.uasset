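; BP_q is a shooting target that awards the first-person player 10 points when a BP_FirstPersonProjectile hits its static mesh.
; On BeginPlay it caches the player character, hides the mesh and reveals it after a random 2 to 15 second timer.
; Each hit adds to the character's Point, hides the mesh and restarts a random reveal timer.
; Hiding changes only visibility, leaving collision untouched.
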(event OnComponentHit(StaticMesh)
  (params (HitComponent :type Primitive%20Component%20Object%20Reference) (OtherActor :type Actor%20Object%20Reference) (OtherComp :type Primitive%20Component%20Object%20Reference) (NormalImpulse :type Vector :default "0, 0, 0") (Hit :type Hit%20Result%20Structure%20%28by%20ref%29))
  (bind _playercharacter (Variables|Default|GetplayerCharacter))
  (Utilities|Casting|CastToBP_FirstPersonProjectile OtherActor)
  (Variables|/Game/FirstPerson/Blueprints/BP_FirstPersonCharacter.BP_FirstPersonCharacter_C|Setpoint _playercharacter (+ (Variables|/Game/FirstPerson/Blueprints/BP_FirstPersonCharacter.BP_FirstPersonCharacter_C|Getpoint _playercharacter) (Variables|Default|GettargetPoint)))
  (Development|SetHiddeninGame (Variables|Default|GetStaticMesh) true false)
  (Utilities|Time|SetTimerbyEvent (delegate Custom|resetTarget) (Math|Random|RandomFloatinRange 2.0 15.0)))

(event Custom|CustomEvent
  (Development|SetHiddeninGame (Variables|Default|GetStaticMesh) false false))

(event Custom|resetTarget
  (Development|SetHiddeninGame (Variables|Default|GetStaticMesh) false false))

(event EventBeginPlay
  (bind _asbp_first_person_character (Utilities|Casting|CastToBP_FirstPersonCharacter (Game|GetPlayerCharacter 0)))
  (Variables|Default|SetplayerCharacter _asbp_first_person_character)
  (Variables|Default|SettargetPoint 10)
  (Development|SetHiddeninGame (Variables|Default|GetStaticMesh) true false)
  (Utilities|Time|SetTimerbyEvent (delegate Custom|CustomEvent) (Math|Random|RandomFloatinRange 2.0 15.0)))

(fn ConstructionScript)